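; Small rocket launcher gun component for modular low-poly robots, built on a parent gun component.
; On construction it binds to the owner robot's fire-activate event, spawns a platform mesh on the robot body at the spawn socket, then attaches the launcher mesh to that platform.
; Each tick it rotates both platform and gun through the RotateGun call.
; The fire event handler is empty, so no firing logic exists here.
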(event `self.ConstructGun`
  (params (RootSocket :type Name))
  (`parent.ConstructGun` RootSocket)
  (add `/Game/RTSGame/Units/BP_RobotBase.FireActivate` (`self.OwnerRobot`) (delegate `fireEvent`))
  (`self.spawnGunMesh` "/Game/RTSGame/ModularLowPolyRobots/Meshes/RobotWeapons/SM_SmallRocketLauncherPlatform.SM_SmallRocketLauncherPlatform" (`/Game/RTSGame/Units/BP_RobotBase.RobotBody` (`self.OwnerRobot`)) (`self.GunPlatform`) (`self.SpawnSocket`))
  (`self.spawnGunMesh` "/Game/RTSGame/ModularLowPolyRobots/Meshes/RobotWeapons/SM_SmallRocketLauncher.SM_SmallRocketLauncher" (`self.GunPlatform`) (`self.GunMesh`) "Any"))

(event `fireEvent`
  (params (value :type Boolean)))

(event `self.ReceiveTick`
  (params (DeltaSeconds :type "Float (single-precision)"))
  (`self.rotateGun` true true))