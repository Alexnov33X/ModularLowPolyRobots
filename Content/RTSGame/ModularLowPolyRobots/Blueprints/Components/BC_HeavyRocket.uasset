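; BC_HeavyRocket is a gun component that mounts a heavy rocket platform on a modular robot.
; On construction it binds to the owner's fire activation, attaches the platform mesh to the robot body, then fills every socket on that platform with a rocket mesh stored in an array.
; Each tick it rotates only the platform, not the gun.
; The fire handler is empty, so no launch logic exists here.
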(event `self.ConstructGun`
  (params (RootSocket :type Name))
  (`parent.ConstructGun` RootSocket)
  (add `/Game/RTSGame/Units/BP_RobotBase.FireActivate` (`self.OwnerRobot`) (delegate `fireEvent`))
  (`self.spawnGunMesh` "/Game/RTSGame/ModularLowPolyRobots/Meshes/RobotWeapons/SM_HeavyRocketPlatform.SM_HeavyRocketPlatform" (`/Game/RTSGame/Units/BP_RobotBase.RobotBody` (`self.OwnerRobot`)) (`self.GunPlatform`) (`self.SpawnSocket`))
  (`self.spawnRockets`))

(event `fireEvent`
  (params (value :type Boolean)))

(event `self.ReceiveTick`
  (params (DeltaSeconds :type "Float (single-precision)"))
  (`self.rotateGun` true))

(fn `spawnRockets`
  (locals (mesh :type "StaticMeshComponent Object Reference") (sockets :type "Array of Name"))
  (bind _output_get (set `local.sockets` (`SceneComponent.GetAllSocketNames` (`self.GunPlatform`))))
  (for _index (range (`KismetArrayLibrary.Array_Length` _output_get))
    (`self.spawnGunMesh` "/Game/RTSGame/ModularLowPolyRobots/Meshes/RobotWeapons/SM_HeavyRocket.SM_HeavyRocket" (`self.GunPlatform`) (`local.mesh`) (`|GetArrayItem` (`local.sockets`) _index))
    (`KismetArrayLibrary.Array_Set` (`self.rocketsMeshes`) _index (`local.mesh`))))