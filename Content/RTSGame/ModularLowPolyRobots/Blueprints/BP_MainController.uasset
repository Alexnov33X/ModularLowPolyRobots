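; BP_MainController is the controller for the Modular Low Poly Robots content, managing a demo menu.
; On BeginPlay, it creates the WB_DemoMenu widget for the local controller and adds it to the viewport.
; Tab and Escape share one FlipFlop that alternately passes true and false to the menu's ShowWidget, starting with true.
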(event `self.ReceiveBeginPlay`
  (if (`self.IsLocalController`)
    (bind _returnvalue (`|CreateWidget` "/Game/RTSGame/ModularLowPolyRobots/Blueprints/Widgets/WB_DemoMenu.WB_DemoMenu_C"))
    (bind _output_get (set `self.DemoMenu` _returnvalue))
    (`UserWidget.AddToViewport` _output_get 0)))

(event `Key|Tab`
  (params (Key :type "Key Structure"))
  (bind _demomenu (`self.DemoMenu`))
  (:`Pressed`
    (`/Engine/EditorBlueprintResources/StandardMacros.FlipFlop` :!label _label
      (:`A`
        (`/Game/RTSGame/ModularLowPolyRobots/Blueprints/Widgets/WB_DemoMenu.ShowWidget` _demomenu true))
      (:`B`
        (`/Game/RTSGame/ModularLowPolyRobots/Blueprints/Widgets/WB_DemoMenu.ShowWidget` _demomenu false)))))

(event `Key|Escape`
  (params (Key :type "Key Structure"))
  (:`Pressed`
    (goto _label)))

(fn `UserConstructionScript`)