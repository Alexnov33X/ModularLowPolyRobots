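; BP_WheelRobot_W6 is a six-wheeled robot vehicle unit that moves on a sphere-trace wheel component.
; Construction registers all six wheel roots as one group simulated on the skeletal mesh.
; Each tick it feeds forward input to that group, averages the wheels' velocity into chassis local velocity, and counter-steers front and rear pairs from smoothed turn input, leaving middle wheels straight.
; A bound brake event passes its value straight to the wheel component.
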(event `self.ReceiveBeginPlay`
  (`parent.ReceiveBeginPlay`)
  (add `self.brakeActivate` (delegate `Brake`)))

(event `Brake` :!signature `self.brakeActivate`
  (params (value :type Boolean))
  (set `/Game/RTSGame/Components/BC_SphereTraceWheel.Brake` value (`self.SphereTraceWheelComponent`)))

(event `self.ReceiveTick`
  (params (DeltaSeconds :type "Float (single-precision)"))
  (`parent.ReceiveTick` DeltaSeconds)
  (`KismetArrayLibrary.Array_Set` (`/Game/RTSGame/Components/BC_SphereTraceWheel.WheelGroupsControlInput` (`self.SphereTraceWheelComponent`)) 0 (`self.MoveForwardAxis`))
  (`self.GetLocalVelocity`)
  (`self.WheelsTurn`))

(fn `GetLocalVelocity`
  (bind _velocity (`self.GetWheelVelocityAverage` (`|MakeArray` (make `/Game/RTSGame/Components/S_FindWheel` 0) (make `/Game/RTSGame/Components/S_FindWheel` 0 1) (make `/Game/RTSGame/Components/S_FindWheel` 0 2) (make `/Game/RTSGame/Components/S_FindWheel` 0 3) (make `/Game/RTSGame/Components/S_FindWheel` 0 4) (make `/Game/RTSGame/Components/S_FindWheel` 0 5))))
  (set `self.ChassisLocalVelocity` _velocity))

(fn `UserConstructionScript`
  (bind _wheeldefaultdistance (`/Game/RTSGame/Components/BC_SphereTraceWheel.WheelDefaultDistance` (`self.SphereTraceWheelComponent`)))
  (`parent.UserConstructionScript`)
  (set `/Game/RTSGame/Components/BC_SphereTraceWheel.WheelsGroups` (`|MakeArray` (make `/Game/RTSGame/Components/S_WheelsGroup` (`|MakeArray` (make `/Game/RTSGame/Components/S_WheelData` :`wheelRootEmpty` (`self.WheelFL`) :`LastContactDistance` _wheeldefaultdistance) (make `/Game/RTSGame/Components/S_WheelData` :`wheelRootEmpty` (`self.WheelFR`) :`LastContactDistance` _wheeldefaultdistance) (make `/Game/RTSGame/Components/S_WheelData` :`wheelRootEmpty` (`self.WheelL`) :`LastContactDistance` _wheeldefaultdistance) (make `/Game/RTSGame/Components/S_WheelData` :`wheelRootEmpty` (`self.WheelR`) :`LastContactDistance` _wheeldefaultdistance) (make `/Game/RTSGame/Components/S_WheelData` :`wheelRootEmpty` (`self.WheelRR`) :`LastContactDistance` _wheeldefaultdistance) (make `/Game/RTSGame/Components/S_WheelData` :`wheelRootEmpty` (`self.WheelRL`) :`LastContactDistance` _wheeldefaultdistance)) 2000.0 2200.0 (`self.SkeletalMesh`))) (`self.SphereTraceWheelComponent`)))

(fn `WheelsTurn`
  (bind _smoothturnvalue (`self.SmoothTurnValue`))
  (`SceneComponent.K2_SetRelativeRotation` (`self.WheelFL`) (`KismetMathLibrary.MakeRotator` 0.0 0.0 (* 20.0 _smoothturnvalue)) false false)
  (`SceneComponent.K2_SetRelativeRotation` (`self.WheelFR`) (`KismetMathLibrary.MakeRotator` 0.0 0.0 (* 20.0 _smoothturnvalue)) false false)
  (`SceneComponent.K2_SetRelativeRotation` (`self.WheelRL`) (`KismetMathLibrary.MakeRotator` 0.0 0.0 (* _smoothturnvalue -20.0)) false false)
  (`SceneComponent.K2_SetRelativeRotation` (`self.WheelRR`) (`KismetMathLibrary.MakeRotator` 0.0 0.0 (* _smoothturnvalue -20.0)) false false))