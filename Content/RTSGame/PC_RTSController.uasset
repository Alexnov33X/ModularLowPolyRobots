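; RTS player controller that creates the HUD widget, drives the RTSCamera view and manages unit selection and orders.
; WASD moves the camera root, the mouse wheel sets clamped spring-arm zoom, and F centers on the first selected unit.
; Left mouse signals selection start/end to the HUD, clearing selection when the trace misses.
; Right-click off a trace target writes the cursor's ground location into each selected unit's Blackboard TargetLocation.
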(event `self.ReceiveBeginPlay`
  (`WidgetBlueprintLibrary.SetInputMode_GameAndUIEx` self null "DoNotLock" false)
  (bind _asrtscamera (cast `/Game/RTSGame/RTSCamera` (`self.GetViewTarget` self)))
  (set `self.RTSCamera` _asrtscamera)
  (bind _returnvalue (`|CreateWidget` "/Game/RTSGame/HUD/W_HUD.W_HUD_C"))
  (bind _output_get (set `self.HUDWidget` _returnvalue))
  (`UserWidget.AddToViewport` _output_get 0))

(event `InputAxisKey|MouseWheelAxis`
  (params (AxisValue :type "Float (single-precision)"))
  (if (`self.IsZoomEnabled`)
    (bind _output_get (set `self.ZoomFactor` (`KismetMathLibrary.FClamp` (+ (* -1 AxisValue) (`self.ZoomFactor`)) 0.0 10.0)))
    (set `SpringArmComponent.TargetArmLength` (+ (* _output_get 200.0) 1000.0) (`/Game/RTSGame/RTSCamera.SpringArm` (`self.RTSCamera`)))))

(event `Key|LeftMouseButton`
  (params (Key :type "Key Structure"))
  (bind _returnvalue (`self.GetHUD`))
  (:`Pressed`
    (message `/Game/RTSGame/BPI_Selection.StartSelection` _returnvalue)
    (if (not (`.ReturnValue` (`self.GetHitResultUnderCursorByChannel` "TraceTypeQuery3")))
      (`self.ClearUnitSelection`)))
  (:`Released`
    (message `/Game/RTSGame/BPI_Selection.EndSelection` _returnvalue)))

(event `Key|RightMouseButton`
  (params (Key :type "Key Structure"))
  (:`Pressed`
    (if (not (`.ReturnValue` (`self.GetHitResultUnderCursorByChannel` "TraceTypeQuery3")))
      (for _array_element (`self.UnitSelection`)
        (`BlackboardComponent.SetValueAsVector` (`AIBlueprintHelperLibrary.GetBlackboard` _array_element) "TargetLocation" (`.Location` (`GameplayStatics.BreakHitResult` (`self.GetHitResultUnderCursorByChannel` "TraceTypeQuery1"))))))))

(event `SetCameraLocation`
  (params (Location :type "Vector Structure"))
  (bind _defaultsceneroot (`/Game/RTSGame/RTSCamera.DefaultSceneRoot` (`self.RTSCamera`)))
  (`KismetSystemLibrary.MoveComponentTo` _defaultsceneroot Location (`SceneComponent.K2_GetComponentRotation` _defaultsceneroot)))

(event `InputAxis|MoveRight`
  (params (AxisValue :type "Float (single-precision)"))
  ;[1 1 1] Управление камеры через WASD, можно дополнить параметром скорости
  (`SceneComponent.K2_AddRelativeLocation` (`/Game/RTSGame/RTSCamera.DefaultSceneRoot` (`self.RTSCamera`)) (* (0.0 50.0 0.0) AxisValue) false false))

(event `Key|F`
  (params (Key :type "Key Structure"))
  ;[1 1 1] Focus Camera
  (:`Pressed`
    (`self.SetCameraLocation` (`self.K2_GetActorLocation` (`|GetArrayItem` (`self.UnitSelection`))))))

(event `InputAxis|MoveForward`
  (params (AxisValue :type "Float (single-precision)"))
  ;[1 1 1] Управление камеры через WASD, можно дополнить параметром скорости
  (`SceneComponent.K2_AddRelativeLocation` (`/Game/RTSGame/RTSCamera.DefaultSceneRoot` (`self.RTSCamera`)) (* (50.0 0.0 0.0) AxisValue) false false))

(fn `AddUnitToSelection`
  (params (Unit :type "/Game/RTSGame/Units/BP_RobotBase Object Reference"))
  (`KismetArrayLibrary.Array_AddUnique` (`self.UnitSelection`) Unit)
  ;[1 1 1] Is selected
  (`/Game/RTSGame/Units/BP_RobotBase.Is Selected` Unit true))

(fn `ClearUnitSelection`
  (bind _unitselection (`self.UnitSelection`))
  ;[1 1 1] Убираем все выделения
  (for _array_element _unitselection
    ;;[1 1 1] is selected off
    (`/Game/RTSGame/Units/BP_RobotBase.Is Selected` _array_element false))
  (`KismetArrayLibrary.Array_Clear` _unitselection)
  (set `self.IsZoomEnabled` true))

(fn `RemoveUnitFromSelection`
  (params (Unit :type "/Game/RTSGame/Units/BP_RobotBase Object Reference"))
  (`KismetArrayLibrary.Array_RemoveItem` (`self.UnitSelection`) Unit)
  ;[1 1 1] is selected off
  (`/Game/RTSGame/Units/BP_RobotBase.Is Selected` Unit false))

(fn `UserConstructionScript`)