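; BP_Bullet is a team-aware projectile for the RTS game that damages what it hits and then bursts.
; Overlapping an actor that is neither another bullet nor tagged with its Team applies Damage and stops ProjectileMovement.
; Tick then grows the sphere as a simple explosion, playing a sound and destroying the bullet at full size, or destroys unhit bullets after a tick-counted lifetime.
; ChangeSpeed sets the forward velocity in local space.
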(event `self.ReceiveBeginPlay`)

(event `self.ReceiveTick`
  (params (DeltaSeconds :type "Float (single-precision)"))
  (bind _timelife (`self.TimeLife`))
  (bind _bulletsize (`self.bulletSize`))
  ;[1 1 1] Explosive anim and destroy bullet
  (set `self.TimeLife` (+ _timelife 1))
  (if (`self.toHit`)
    (if (== _bulletsize 0.5)
      (`PrimitiveComponent.SetCollisionEnabled` (`self.Sphere`) "NoCollision"))
    (bind _output_get (set `self.bulletSize` (* _bulletsize 1.3)))
    (`SceneComponent.SetWorldScale3D` (`self.Sphere`) (`KismetMathLibrary.Conv_DoubleToVector` _output_get))
    (if (> _output_get 4.0)
      (`GameplayStatics.PlaySoundAtLocation` "/Game/CSC/Demo/Sounds/bum_sm_3.bum_sm_3" (`SceneComponent.K2_GetComponentLocation` (`self.Sphere`)) (struct) 0.4 1.0 0.0 null null null)
      (`self.K2_DestroyActor` :!label _label))
    (elif (> _timelife 150)
      (goto _label))))

(event `self.Sphere.OnComponentBeginOverlap`
  (params (OverlappedComponent :type "PrimitiveComponent Object Reference") (OtherActor :type "Actor Object Reference") (OtherComp :type "PrimitiveComponent Object Reference") (OtherBodyIndex :type Integer) (bFromSweep :type Boolean) (SweepResult :type "HitResult Structure (by ref)"))
  ;[1 1 1] Detect hit to enemy tag
  (cast `/Game/RTSGame/BP_Bullet` OtherActor
    (:`CastFailed`
      (if (and (> (`self.TimeLife`) 2) (not (`self.ActorHasTag` OtherActor (`self.Team`))))
        (set `self.toHit` true :!label _label_2)
        (`GameplayStatics.ApplyDamage` OtherActor (`self.Damage`))
        (set `MovementComponent.Velocity` (0.0 0.0 0.0) (`self.ProjectileMovement`))
        (elif (not (`self.ActorHasTag` OtherActor (`self.Team`)))
          (goto _label_2))))))

(fn `ChangeSpeed`
  (params (NewSpeed :type "Float (double-precision)"))
  (`ProjectileMovementComponent.SetVelocityInLocalSpace` (`self.ProjectileMovement`) (`KismetMathLibrary.MakeVector` NewSpeed)))

(fn `UserConstructionScript`)